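; CubeBP is a moving hazard cube that sends the game to the YouDie level on any overlap or hit.
; On BeginPlay it finds a SplintPath actor and runs a timeline that lerps distance along its spline to set the cube's world location, with TimeToComplete scaling the play rate.
; Rotation is always sampled at the spline's start in local space, so it does not follow the curve.
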(event `self.ReceiveBeginPlay`
  (bind _returnvalue (`GameplayStatics.GetActorOfClass` "/Game/CustomCollecion/Blueprint/AI/SplintPath.SplintPath_C"))
  (set `self.Splint Refer` _returnvalue)
  (`self.Move Object`))

(event `Move Object`
  (bind _spline (`/Game/CustomCollecion/Blueprint/AI/SplintPath.Spline` (`self.Splint Refer`)))
  (`TimelineComponent.SetPlayRate` (`self.Move Object T`) (/ 0.05 (`self.TimeToComplete`)))
  (bind (_direction _move_track) (`Timeline|Move Object T`)
    (:`Update`
      (`self.K2_SetActorTransform` (`KismetMathLibrary.MakeTransform` (`SplineComponent.GetLocationAtDistanceAlongSpline` _spline (`KismetMathLibrary.Lerp` 0.0 (`SplineComponent.GetSplineLength` (`/Game/CustomCollecion/Blueprint/AI/SplintPath.Spline` (`self.Splint Refer`))) _move_track) "World") (`SplineComponent.GetRotationAtDistanceAlongSpline` _spline 0.0 "Local"))))))

(event `self.Cube.OnComponentBeginOverlap`
  (params (OverlappedComponent :type "PrimitiveComponent Object Reference") (OtherActor :type "Actor Object Reference") (OtherComp :type "PrimitiveComponent Object Reference") (OtherBodyIndex :type Integer) (bFromSweep :type Boolean) (SweepResult :type "HitResult Structure (by ref)"))
  (`KismetSystemLibrary.PrintString` "You dead" :!label _label)
  (`GameplayStatics.OpenLevel` "YouDie"))

(event `self.Cube.OnComponentHit`
  (params (HitComponent :type "PrimitiveComponent Object Reference") (OtherActor :type "Actor Object Reference") (OtherComp :type "PrimitiveComponent Object Reference") (NormalImpulse :type "Vector Structure") (Hit :type "HitResult Structure (by ref)"))
  (goto _label))

(fn `UserConstructionScript`)